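; BP_Bullet is a projectile that damages either the player or enemies, depending on its TargetType.
; Construction feeds Speed into the ProjectileMovement initial speed, and BeginPlay tints the Sphere through a dynamic material by target type.
; On overlap with an actor of exactly the target class, it applies fixed damage, destroys itself and prints the hit.
; An older switch-based damage branch remains unconnected.
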(event `self.ReceiveBeginPlay`
  (bind _sphere (`self.Sphere`))
  (bind _returnvalue (`PrimitiveComponent.CreateDynamicMaterialInstance` _sphere 0 (`PrimitiveComponent.GetMaterial` _sphere 0) "None"))
  (`MaterialInstanceDynamic.SetVectorParameterValue` _returnvalue "Color" (select `/Game/Blueprint/Bullet/E_TargetType` (`self.TargetType`) :`NewEnumerator0` (struct :`R` 1.0 :`G` 0.099899 :`B` 0.099899 :`A` 1.0) :`NewEnumerator1` (struct :`R` 0.099899 :`G` 0.281498 :`B` 1.0 :`A` 1.0) :!type "LinearColor Structure")))

(event `self.ReceiveActorBeginOverlap`
  (params (OtherActor :type "Actor Object Reference"))
  ; Check if overlapped actor is the same class as target class
  (if (== (`GameplayStatics.GetObjectClass` OtherActor) (select `/Game/Blueprint/Bullet/E_TargetType` (`self.TargetType`) :`NewEnumerator0` "/Game/Blueprint/Player/BP_player.BP_player_C" :`NewEnumerator1` "/Game/Blueprint/Enemies/Enemy/BP_Enemy.BP_Enemy_C" :!type "Object Class Reference"))
    (bind _returnvalue (`GameplayStatics.ApplyDamage` OtherActor 10.0 (`self.GetInstigatorController`) self))
    (`self.K2_DestroyActor`)
    (`KismetSystemLibrary.PrintString` (`KismetStringLibrary.Concat_StrStr` "Target hit for " (`KismetStringLibrary.Conv_DoubleToString` _returnvalue) " damage"))))

(fn `UserConstructionScript`
  (set `ProjectileMovementComponent.InitialSpeed` (`self.Speed`) (`self.ProjectileMovement`)))