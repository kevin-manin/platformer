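; Shop character actor that lets the player open the shop while standing inside its sphere trigger.
; Entering the sphere sets CanOpenShop on BP_player and shows a WBP_InteractWithShop widget; leaving clears the flag and removes the stored widget.
; Disconnected leftover nodes for opening WBP_Shop with pause and mouse cursor, and for closing widgets, never run, so this Blueprint does not open the shop itself.
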(event `self.Sphere.OnComponentBeginOverlap`
  (params (OverlappedComponent :type "PrimitiveComponent Object Reference") (OtherActor :type "Actor Object Reference") (OtherComp :type "PrimitiveComponent Object Reference") (OtherBodyIndex :type Integer) (bFromSweep :type Boolean) (SweepResult :type "HitResult Structure (by ref)"))
  (bind _asbp_player (cast `/Game/Blueprint/Player/BP_player` OtherActor))
  (set `/Game/Blueprint/Player/BP_player.CanOpenShop` true _asbp_player)
  (bind _returnvalue (`|CreateWidget` "/Game/Screens/HUD/WBP_InteractWithShop.WBP_InteractWithShop_C"))
  (set `self.InteractWidgetRef` _returnvalue)
  (`UserWidget.AddToViewport` _returnvalue 0))

(event `self.Sphere.OnComponentEndOverlap`
  (params (OverlappedComponent :type "PrimitiveComponent Object Reference") (OtherActor :type "Actor Object Reference") (OtherComp :type "PrimitiveComponent Object Reference") (OtherBodyIndex :type Integer))
  (bind _interactwidgetref (`self.InteractWidgetRef`))
  (bind _asbp_player (cast `/Game/Blueprint/Player/BP_player` OtherActor))
  (set `/Game/Blueprint/Player/BP_player.CanOpenShop` false _asbp_player)
  (if (`KismetSystemLibrary.IsValid` _interactwidgetref)
    (`/Game/Screens/HUD/WBP_InteractWithShop.RemoveWidget` _interactwidgetref)))

(fn `UserConstructionScript`)