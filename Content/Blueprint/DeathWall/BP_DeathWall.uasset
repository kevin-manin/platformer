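; A death wall actor that travels along a spline and deals heavy damage to the player character on overlap.
; While active, Tick advances the distance by wall speed and sweeps the mesh to that spline point, following its location, yaw and scale.
; A reset event returns the wall to the spline start, without applying spline scale, and deactivates it; activation is not handled in this graph.
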(event `self.ReceiveActorBeginOverlap`
  (params (OtherActor :type "Actor Object Reference"))
  (bind _returnvalue (`GameplayStatics.GetPlayerCharacter` 0))
  ; Deal damage on collision
  (if (== OtherActor _returnvalue)
    (`GameplayStatics.ApplyDamage` _returnvalue 1000.0 null self)))

(event `self.ReceiveTick`
  (params (DeltaSeconds :type "Float (single-precision)"))
  (bind _returnvalue (`SplineComponent.GetTransformAtDistanceAlongSpline` (`self.Spline`) (`self.DistanceAlongSpline`) "Local" true))
  ; Move wall along Spline
  (if (`self.IsActive`)
    (set `self.DistanceAlongSpline` (+ (* DeltaSeconds (`self.WallSpeed`)) (`self.DistanceAlongSpline`)))
    (`SceneComponent.K2_SetRelativeTransform` (`self.SM_DeathWall`) (`KismetMathLibrary.MakeTransform` (.location _returnvalue) (`KismetMathLibrary.MakeRotator` 0.0 0.0 (.yaw (.rotation _returnvalue))) (.scale _returnvalue)) true false)))

(event `self.K2_OnReset`
  (bind _returnvalue (`SplineComponent.GetTransformAtDistanceAlongSpline` (`self.Spline`) (`self.DistanceAlongSpline`) "Local" false))
  ; Wall Reset
  (set `self.DistanceAlongSpline` 0.0)
  (`SceneComponent.K2_SetRelativeTransform` (`self.SM_DeathWall`) (`KismetMathLibrary.MakeTransform` (.location _returnvalue) (`KismetMathLibrary.MakeRotator` 0.0 0.0 (.yaw (.rotation _returnvalue)))) false false)
  (set `self.IsActive` false))

(fn `UserConstructionScript`)