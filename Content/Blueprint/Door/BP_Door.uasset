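; BP_Door is a door actor that opens through a Level Sequence cutscene and then hands control back to the player.
; PlayDoorSequence prints a debug string, creates and plays a player for DoorSequence, and binds PossesPlayer to its finish.
; PossesPlayer teleport-free raises the Door component without sweep, repossesses the player pawn, restores game-only input and clears BP_player's Invulnerability.
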(event `PlayDoorSequence`
  (`KismetSystemLibrary.PrintString` "Hello")
  (bind (_outactor _returnvalue) (`LevelSequencePlayer.CreateLevelSequencePlayer` (`self.DoorSequence`)))
  (`MovieSceneSequencePlayer.Play` _returnvalue)
  (add `MovieSceneSequencePlayer.OnFinished` _returnvalue (delegate `PossesPlayer`)))

(event `PossesPlayer`
  (bind _returnvalue (`GameplayStatics.GetPlayerController` 0))
  (bind _door (`self.door`))
  (`SceneComponent.K2_SetWorldLocation` _door (+ (`SceneComponent.K2_GetComponentLocation` _door) (0.0 0.0 500.0)) false false)
  (`Controller.Possess` _returnvalue (`GameplayStatics.GetPlayerPawn` 0))
  (`WidgetBlueprintLibrary.SetInputMode_GameOnly` _returnvalue)
  (bind _asbp_player (cast `/Game/Blueprint/Player/BP_player` (`GameplayStatics.GetPlayerPawn` 0)))
  (set `/Game/Blueprint/Player/BP_player.Invulnerability` false _asbp_player))

(fn `UserConstructionScript`)