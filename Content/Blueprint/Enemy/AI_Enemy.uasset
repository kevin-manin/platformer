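; Enemy AI controller that runs the BT_Enemy behavior tree and feeds it sight perception of the player.
; On each perception update it ignores non-sight stimuli and any actor other than player character 0.
; It sets the TargetPlayer blackboard key while the player is seen and clears it when sight is lost, also storing the stimulus position as LastKnownLocation.
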(event `self.ReceiveBeginPlay`
  (`self.RunBehaviorTree` "/Game/Blueprint/Enemy/BT_Enemy.BT_Enemy"))

(event `self.AIPerception.OnTargetPerceptionUpdated`
  (params (Actor :type "Actor Object Reference") (Stimulus :type "AIStimulus Structure"))
  (`self.HandleSightSense` Actor Stimulus))

(fn `HandleSightSense`
  (params (Actor :type "Actor Object Reference") (Stimulus :type "AIStimulus Structure"))
  (bind _blackboard (`self.Blackboard`))
  (bind (_stimulus_age _stimulus_expirationage _stimulus_strength _stimulus_stimuluslocation _stimulus_receiverlocation _stimulus_tag _stimulus_bsuccessfullysensed) (break `AIStimulus` (`local.Stimulus`)))
  (bind _returnvalue (`AIPerceptionSystem.GetSenseClassForStimulus` Stimulus))
  (if (== _returnvalue "/Script/AIModule.AISense_Sight")
    (if (== (`local.Actor`) (`GameplayStatics.GetPlayerCharacter` 0))
      (`BlackboardComponent.SetValueAsObject` _blackboard "TargetPlayer" (`KismetMathLibrary.SelectObject` (`local.Actor`) null _stimulus_bsuccessfullysensed))
      (if (not _stimulus_bsuccessfullysensed)
        (`BlackboardComponent.SetValueAsVector` _blackboard "LastKnownLocation" _stimulus_stimuluslocation))
      (else
        (return)))
    (else
      (return))))

(fn `UserConstructionScript`)