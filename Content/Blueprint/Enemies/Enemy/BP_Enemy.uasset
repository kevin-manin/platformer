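; BP_Enemy is an enemy actor that dies from any single instance of damage and counts toward the kill total.
; On BeginPlay it waits briefly, then casts and caches BP_GameInstance.
; AnyDamage increments EnemiesKilled on that instance and destroys the actor, regardless of damage amount or causer.
; A check that the damage causer is the player character exists but is disconnected, so it never runs.
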(event `self.ReceiveBeginPlay`
  (`KismetSystemLibrary.Delay` 0.2)
  (bind _asbp_game_instance (cast `/Game/Blueprint/GameInstance/BP_GameInstance` (`GameplayStatics.GetGameInstance`)))
  (set `self.GameInstance` _asbp_game_instance))

(event `self.ReceiveAnyDamage`
  (params (Damage :type "Float (single-precision)") (DamageType :type "DamageType Object Reference") (InstigatedBy :type "Controller Object Reference") (DamageCauser :type "Actor Object Reference"))
  (`/Engine/EditorBlueprintResources/StandardMacros.IncrementInt` (`/Game/Blueprint/GameInstance/BP_GameInstance.EnemiesKilled` (`self.GameInstance`))
    (:`  `
      (`self.K2_DestroyActor`))))

(fn `UserConstructionScript`)