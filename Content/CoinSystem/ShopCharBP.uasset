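; ShopCharBP is a shop actor in the coin system that gives the player access to the shop interface by proximity.
; When BP_player enters its Sphere, it creates a WBP_Shop widget, adds it to the viewport and shows the mouse cursor.
; When the player leaves, it finds top-level widgets by class, removes them from their parent and hides the cursor.
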(event `self.Sphere.OnComponentBeginOverlap`
  (params (OverlappedComponent :type "PrimitiveComponent Object Reference") (OtherActor :type "Actor Object Reference") (OtherComp :type "PrimitiveComponent Object Reference") (OtherBodyIndex :type Integer) (bFromSweep :type Boolean) (SweepResult :type "HitResult Structure (by ref)"))
  (cast `/Game/Blueprint/Player/BP_player` OtherActor)
  (bind _returnvalue (`|CreateWidget` "/Game/CoinSystem/WBP_Shop.WBP_Shop_C"))
  (`UserWidget.AddToViewport` _returnvalue 0)
  (set `PlayerController.bShowMouseCursor` true (`GameplayStatics.GetPlayerController` 0)))

(event `self.Sphere.OnComponentEndOverlap`
  (params (OverlappedComponent :type "PrimitiveComponent Object Reference") (OtherActor :type "Actor Object Reference") (OtherComp :type "PrimitiveComponent Object Reference") (OtherBodyIndex :type Integer))
  (cast `/Game/Blueprint/Player/BP_player` OtherActor)
  (bind _foundwidgets (`WidgetBlueprintLibrary.GetAllWidgetsOfClass` (`self.Widget Class`)))
  (`Widget.RemoveFromParent` _foundwidgets)
  (set `PlayerController.bShowMouseCursor` false (`GameplayStatics.GetPlayerController` 0)))

(fn `UserConstructionScript`)