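; Moving platform Blueprint that shifts its Cube back and forth along a Timeline, starting at BeginPlay.
; Each Timeline update sets the Cube's relative location from the Moving vector track, with no sweep.
; The same update runs into a five-second Delay, after which the IsLooped flag toggles and alternately reverses or plays the Timeline.
; The direction flip hangs off Update rather than Finished, so the Delay sets its timing.
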(event `self.ReceiveBeginPlay`
  (bind (_direction _moving) (`Timeline|Timeline` :!label _label)
    (:`Update`
      (bind _result (`/Engine/EditorBlueprintResources/StandardMacros.NegateFloat` (.x _moving))
        (:`  `
          (`SceneComponent.K2_SetRelativeLocation` (`self.Cube`) (`KismetMathLibrary.MakeVector` _result (.y _moving) (.z _moving)) false false)
          (`KismetSystemLibrary.Delay` 5.0)
          (if (`self.IsLooped`)
            (set `self.IsLooped` false)
            (goto _label)
            (else
              (set `self.IsLooped` true)
              (goto _label :!via `Reverse`))))))))

(fn `UserConstructionScript`)